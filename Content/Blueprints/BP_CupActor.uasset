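; BP_CupActor is a cup formation actor that fills stage points with BP_Cup child actors and listens for balls landing in them.
; Its construction script destroys previous cups, then snaps a new child actor to each child of FirstStage and stores that point as the cup's CupParent.
; BeginPlay binds every cup's ball-entered event, whose handler only prints a debug string.
; SecondStage and FinalStage are unused.
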(event Custom|BallEnteredACup
  (params (Scene :type Scene%20Component%20Object%20Reference) (Cup :type BP%20Cup%20Object%20Reference))
  (Development|PrintString "Hello"))

(event EventBeginPlay
  (for _array_element (Variables|Default|GetCups)
    (bind _asbp_cup (Utilities|Casting|CastToBP_Cup (Variables|/Script/Engine.ChildActorComponent|GetChildActor _array_element)))
    (EventDispatchers|BindEventtoBallEnteredCup _asbp_cup (EventDispatchers|CreateEvent :!event Custom|BallEnteredACup))))

(event Collision|EventActorBeginOverlap
  (params (OtherActor :type Actor%20Object%20Reference)))

(event EventTick
  (params (DeltaSeconds :type Float%20%28single-precision%29)))

(fn ConstructionScript
  (for _array_element (Variables|Default|GetCups)
    (Components|DestroyComponent _array_element))
  (for _array_element_2 (Components|GetChildrenComponents (Variables|Default|GetFirstStage) false)
    (bind _returnvalue (AddComponent|AddChildActorComponent true))
    (Transformation|AttachComponentToComponent _returnvalue _array_element_2 "None" "SnapToTarget" "SnapToTarget" "KeepWorld" true)
    (Transformation|SetRelativeTransform _returnvalue (Math|Transform|MakeTransform "0, 0, 0") false false)
    (Utilities|Array|Add (Variables|Default|GetCups) _returnvalue)
    (bind _asbp_cup (Utilities|Casting|CastToBP_Cup (Variables|/Script/Engine.ChildActorComponent|GetChildActor _returnvalue)))
    (Variables|/Game/Blueprints/BP_Cup.BP_Cup_C|SetCupParent _asbp_cup _array_element_2)))