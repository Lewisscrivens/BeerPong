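; BP_BeerPongPawn is a beer pong pawn that lets the player drag a child-actor ball with the mouse.
; Left click enables ball physics, grabs it with a PhysicsHandle, records mouse and ball start positions, and starts a looping timer.
; UpdateGrabHandle converts mouse offset into a target along the Up and Left components' forward vectors, scaled by MaxMovement.
; Releasing the button clears the UpdateGrabHandle timer and lets go of the ball.
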(event Custom|UpdateGrabHandle
  (bind _maxmovement (Variables|Default|GetmaxMovement))
  (bind _returnvalue (Class|WidgetLayoutLibrary|GetMousePositiononViewport))
  (Class|PhysicsHandleComponent|SetTargetLocationandRotation (Variables|Default|GetPhysicsHandle) (+ (Variables|Default|GetOriginalWorldLoc) (* (Math|Vector|GetForwardVector (Variables|Default|GetUp)) (* (/ (.y (- (Variables|Default|GetMouseOriginalOffset) _returnvalue)) 5e+02) _maxmovement)) (* (Math|Vector|GetForwardVector (Variables|Default|GetLeft)) (* (/ (.x (- (Variables|Default|GetMouseOriginalOffset) _returnvalue)) 5e+02) _maxmovement))) "0, 0, 0"))

(event EventBeginPlay)

(event Collision|EventActorBeginOverlap
  (params (OtherActor :type Actor%20Object%20Reference)))

(event EventTick
  (params (DeltaSeconds :type Float%20%28single-precision%29)))

(event Input|MouseEvents|LeftMouseButton
  (params (Key :type Key%20Structure :default "None"))
  (bind _ball (Variables|Default|GetBall))
  (bind _ballmesh (Variables|/Game/Blueprints/BP_Ball.BP_Ball_C|GetBallMesh _ball))
  (bind _returnvalue (Transformation|GetWorldTransform _ballmesh))
  (:Pressed
    (Utilities|Time|SetTimerbyEvent (EventDispatchers|CreateEvent :!event Custom|UpdateGrabHandle) 0.02 true)
    (Physics|SetSimulatePhysics _ballmesh true)
    (Physics|Components|PhysicsHandle|GrabComponentatLocationwithRotation (Variables|Default|GetPhysicsHandle) _ballmesh "None" (.location _returnvalue) (.rotation _returnvalue))
    (bind _returnvalue_2 (Class|WidgetLayoutLibrary|GetMousePositiononViewport))
    (Variables|Default|SetMouseOriginalOffset _returnvalue_2)
    (Variables|Default|SetOriginalWorldLoc (.location _returnvalue)))
  (:Released
    (Utilities|Time|ClearTimerbyFunctionName self "UpdateGrabHandle")
    (Physics|Components|PhysicsHandle|ReleaseComponent (Variables|Default|GetPhysicsHandle))))

(fn ConstructionScript
  (bind _asbp_ball (Utilities|Casting|CastToBP_Ball (Variables|/Script/Engine.ChildActorComponent|GetChildActor (Variables|Default|GetChildActor))))
  (Variables|Default|SetBall _asbp_ball))